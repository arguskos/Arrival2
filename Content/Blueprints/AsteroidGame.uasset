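; Game-flow Blueprint for an asteroid game that shows the score widget and reacts to ship and asteroid destruction events.
; Destroyed asteroids spawn an explosion actor at their location.
; A ship hit reopens the "Test" level when lives are zero; otherwise it hides the pawn by zeroing its scale.
; A short timer then teleports the pawn to the world origin, restores its scale and clears the BaseShip dead flag.
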(event `self.ReceiveBeginPlay`
  (bind _returnvalue (`|CreateWidget` "/Game/Blueprints/ScoreWidget.ScoreWidget_C"))
  (`UserWidget.AddToViewport` _returnvalue 0)
  (add `self.AsteroidDestroyed` (delegate `OnAsteroidDestroyed`))
  (add `self.ShipDestroyed` (delegate `OnShipHit`)))

(event `OnShipHit`
  (if (== (`self.GetLives`) 0)
    (`GameplayStatics.OpenLevel` "Test")
    (else
      (`self.SetActorScale3D` (`GameplayStatics.GetPlayerPawn` 0) (0.0 0.0 0.0))
      (`KismetSystemLibrary.K2_SetTimerDelegate` (delegate `Respawn`) 1.0))))

(event `OnAsteroidDestroyed` :!signature `self.AsteroidDestroyed`
  (params (Actor :type "BaseAsteroid Object Reference"))
  (`|SpawnActorFromClass` "/Game/Blueprints/B_Explosion.B_Explosion_C" (`KismetMathLibrary.Conv_VectorToTransform` (`self.K2_GetActorLocation` Actor)) "Undefined" "OverrideRootScale" null null))

(event `Respawn`
  (bind _returnvalue (`GameplayStatics.GetPlayerPawn` 0))
  (`self.K2_SetActorLocation` _returnvalue (0.0 0.0 0.0) false true)
  (`self.SetActorScale3D` _returnvalue (1.0 1.0 1.0))
  (bind _asbase_ship (cast `BaseShip` _returnvalue))
  (`BaseShip.SetIsDead` _asbase_ship false))

(fn `UserConstructionScript`)